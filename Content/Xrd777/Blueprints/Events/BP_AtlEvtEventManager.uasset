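; Event manager actor that starts the AtlEvt event matching the current level and drives a test message UI for it.
; On BeginPlay it parses category and major/minor IDs from the underscore-delimited level name, then calls the event through AtlEvtSubsystem.
; Its events feed WBP_MessageUITest with dialogue, selection buttons and debug text.
; Bustup previews layer pose, eye and mouth textures from BustupExistDataAsset through dynamic materials.
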(event `self.ReceiveBeginPlay`
  (bind _returnvalue (subsystem `AtlEvtSubsystem`))
  (bind _eventtype (`self.EventType`))
  (bind _eventmajor (`self.EventMajor`))
  (bind _eventminor (`self.EventMinor`))
  (bind _returnvalue_2 (`GameplayStatics.GetCurrentLevelName` true))
  (for (_array_element _array_index) (`KismetStringLibrary.ParseIntoArray` _returnvalue_2 "_")
    (switch `int` _array_index
      (:`2`
        (switch `string` (`KismetStringLibrary.ToLower` _array_element)
          (:`Default`
            (set `self.EventType` "CMMU" :!label _label))
          (:`main`
            (set `self.EventType` "MAIN"))
          (:`cmmu`
            (goto _label))
          (:`qest`
            (set `self.EventType` "MAIN"))
          (:`extr`
            (set `self.EventType` "MAIN"))
          (:`fild`
            (set `self.EventType` "FILD"))))
      (:`3`
        (set `self.EventMajor` (`KismetStringLibrary.Conv_StringToInt` _array_element)))
      (:`4`
        (set `self.EventMinor` (`KismetStringLibrary.Conv_StringToInt` _array_element)))))
  (set `self.EventRankVisible` (`.EventRank` (break `AtlEvtPreData` (`AtlEvtSubsystem.GetEvtPreData` _returnvalue _eventtype _eventmajor _eventminor))))
  (`AtlEvtSubsystem.CallCategoryEvent` _returnvalue _eventtype _eventmajor _eventminor (`self.EventParam`))
  (bind _returnvalue_3 (`|CreateWidget` "/Game/Xrd777/Test/Rirurin/WBP_MessageUITest.WBP_MessageUITest_C"))
  (bind _output_get (set `self.MessageUITest` _returnvalue_3))
  (set `/Game/Xrd777/Test/Rirurin/WBP_MessageUITest.Owner` self _output_get)
  (`Widget.SetVisibility` (`/Game/Xrd777/Test/Rirurin/WBP_MessageUITest.MsgDebugInfo` _output_get) "Hidden")
  (`UserWidget.AddToViewport` _output_get 0))

(event `self.ReceiveDrawMessage`
  (params (MessageText :type String) (SpeakerText :type String))
  (bind _messageuitest (`self.MessageUITest`))
  (bind _speakertext (`/Game/Xrd777/Test/Rirurin/WBP_MessageUITest.SpeakerText` _messageuitest))
  (`Widget.SetVisibility` (`/Game/Xrd777/Test/Rirurin/WBP_MessageUITest.MsgBox` _messageuitest) "Visible")
  (`Widget.SetVisibility` (`/Game/Xrd777/Test/Rirurin/WBP_MessageUITest.NextMsgBtn` _messageuitest) "Visible")
  (if (`KismetStringLibrary.IsEmpty` SpeakerText)
    (`TextBlock.SetText` _speakertext "")
    (else
      (`TextBlock.SetText` _speakertext (`KismetTextLibrary.Conv_StringToText` SpeakerText))))
  (`TextBlock.SetText` (`/Game/Xrd777/Test/Rirurin/WBP_MessageUITest.MsgText` _messageuitest) (`KismetTextLibrary.Conv_StringToText` MessageText)))

(event `self.ReceiveTick`
  (params (DeltaSeconds :type "Float (single-precision)"))
  (bind _returnvalue (`self.CreateEventDebugText` (`|GetEnumeratorNameAsString` (`self.EventType`)) (`self.EventMajor`) (`self.EventMinor`) (`self.EventRankVisible`)))
  (`TextBlock.SetText` (`/Game/Xrd777/Test/Rirurin/WBP_MessageUITest.DebugInfo` (`self.MessageUITest`)) (`KismetTextLibrary.Conv_StringToText` _returnvalue)))

(event `self.ReceiveUpdateMsgDebug`
  (params (DebugText :type String) (bVisibility :type Boolean))
  (bind _msgdebuginfo (`/Game/Xrd777/Test/Rirurin/WBP_MessageUITest.MsgDebugInfo` (`self.MessageUITest`)))
  (if bVisibility
    (`Widget.SetVisibility` _msgdebuginfo "Visible")
    (else
      (`Widget.SetVisibility` _msgdebuginfo "Hidden")))
  (`TextBlock.SetText` _msgdebuginfo (`KismetTextLibrary.Conv_StringToText` DebugText)))

(event `self.ReceiveDrawBustup`
  (params (CharacterId :type Integer) (a2 :type Integer) (a3 :type Integer) (a4 :type Integer) (a5 :type Integer) (a6 :type Integer))
  (bind _messageuitest (`self.MessageUITest`))
  ;[1 1 1] Get Bustup Exist Data Asset
  (bind _returnvalue (`AssetRegistry.GetAssetByObjectPath` (`AssetRegistryHelpers.GetAssetRegistry`) "/Game/Xrd777/UI/Tables/BustupExistDataAsset.BustupExistDataAsset" false))
  (if (`AssetRegistryHelpers.IsValid` _returnvalue)
    (bind _asbustup_exist_data_asset (cast `BustupExistDataAsset` (`AssetRegistryHelpers.GetAsset` _returnvalue)))
    (bind (_pose _eyepartsid _mouthpartsid _eyepos _mouthpos _blushpos _sweatpos _offset _clothout _returnvalue_2) (`BustupExistDataAsset.GetBustupParameters` _asbustup_exist_data_asset CharacterId a2 a3))
    (if _returnvalue_2
      (bind _returnvalue_3 (`BustupExistDataAsset.GetPoseTexture` _asbustup_exist_data_asset CharacterId _clothout _pose))
      (`self.BustupPartSetTexture` (`/Game/Xrd777/Test/Rirurin/WBP_MessageUITest.BustupPoseMID` _messageuitest) (`/Game/Xrd777/Test/Rirurin/WBP_MessageUITest.BustupPose` _messageuitest) _returnvalue_3 (0.0 0.0))
      (bind _returnvalue_4 (`BustupExistDataAsset.GetEyeTexture` _asbustup_exist_data_asset CharacterId a2 _eyepartsid 1))
      (`self.BustupPartSetTexture` (`/Game/Xrd777/Test/Rirurin/WBP_MessageUITest.BustupEyeMID` _messageuitest) (`/Game/Xrd777/Test/Rirurin/WBP_MessageUITest.BustupEyes` _messageuitest) _returnvalue_4 _eyepos)
      (bind _returnvalue_5 (`BustupExistDataAsset.GetMouthTexture` _asbustup_exist_data_asset CharacterId a2 _mouthpartsid 1))
      (`self.BustupPartSetTexture` (`/Game/Xrd777/Test/Rirurin/WBP_MessageUITest.BustupMouthMID` _messageuitest) (`/Game/Xrd777/Test/Rirurin/WBP_MessageUITest.BustupMouth` _messageuitest) _returnvalue_5 _mouthpos)
      (else
        (`KismetSystemLibrary.PrintString` (`KismetStringLibrary.Concat_StrStr` "WARNING: Bustup for character " (`KismetStringLibrary.Conv_IntToString` CharacterId) ", face" (`KismetStringLibrary.Conv_IntToString` a2) " is missing!"))))
    (else
      (`KismetSystemLibrary.PrintString` "ERROR: Can't get bustup exist data asset!!! Bustup preview won't work!!!"))))

(event `self.ReceiveClearBustup`
  (bind _messageuitest (`self.MessageUITest`))
  (`Widget.SetVisibility` (`/Game/Xrd777/Test/Rirurin/WBP_MessageUITest.BustupPose` _messageuitest) "Hidden")
  (`Widget.SetVisibility` (`/Game/Xrd777/Test/Rirurin/WBP_MessageUITest.BustupEyes` _messageuitest) "Hidden")
  (`Widget.SetVisibility` (`/Game/Xrd777/Test/Rirurin/WBP_MessageUITest.BustupMouth` _messageuitest) "Hidden"))

(event `self.ReceiveClearMessageBox`
  (bind _messageuitest (`self.MessageUITest`))
  (`Widget.SetVisibility` (`/Game/Xrd777/Test/Rirurin/WBP_MessageUITest.MsgBox` _messageuitest) "Hidden")
  (`Widget.SetVisibility` (`/Game/Xrd777/Test/Rirurin/WBP_MessageUITest.NextMsgBtn` _messageuitest) "Hidden"))

(event `self.ReceiveCreateSelectOptions`
  (params (SelOptions :type "Array of String (by ref)"))
  (bind _messageuitest (`self.MessageUITest`))
  (`Widget.SetVisibility` (`/Game/Xrd777/Test/Rirurin/WBP_MessageUITest.NextMsgBtn` _messageuitest) "Hidden")
  (for (_array_element _array_index) SelOptions
    (bind _returnvalue (`|CreateWidget` "/Game/Xrd777/Test/Rirurin/WBP_MessageSelection.WBP_MessageSelection_C"))
    (set `/Game/Xrd777/Test/Rirurin/WBP_MessageSelection.Owner` _messageuitest _returnvalue)
    (`KismetArrayLibrary.Array_Add` (`/Game/Xrd777/Test/Rirurin/WBP_MessageUITest.SelOptions` _messageuitest) _returnvalue)
    (set `/Game/Xrd777/Test/Rirurin/WBP_MessageSelection.SelIndex` _array_index _returnvalue)
    (`TextBlock.SetText` (`/Game/Xrd777/Test/Rirurin/WBP_MessageSelection.SelButtonLabel` _returnvalue) (`KismetTextLibrary.Conv_StringToText` _array_element))
    (`PanelWidget.AddChild` (`/Game/Xrd777/Test/Rirurin/WBP_MessageUITest.MsgBtnList` _messageuitest) _returnvalue)))

(event `self.ReceiveSetLocalDataBP`
  (params (Index :type Integer) (Data :type Integer))
  (`AtlEvtSubsystem.SetLocalData` (subsystem `AtlEvtSubsystem`) Index Data))

(fn `BustupPartSetTexture`
  (params (Mid :type "MaterialInstanceDynamic Object Reference (by ref)") (Image :type "Image Object Reference (by ref)") (Tex :type "Texture2D Object Reference") (Offset :type "Vector2D Structure") (ImageType :type Integer))
  (bind _returnvalue (`Texture2D.Blueprint_GetSizeY` Tex))
  (bind (_x _y) (`KismetMathLibrary.BreakVector2D` (/ Offset 3.0)))
  (bind _returnvalue_2 (`KismetMaterialLibrary.CreateDynamicMaterialInstance` "/Game/Xrd777/Test/Rirurin/MM_BustupDraw.MM_BustupDraw"))
  (`|VariableSetRef` Mid _returnvalue_2)
  (`Image.SetBrush` Image (`WidgetBlueprintLibrary.MakeBrushFromMaterial` _returnvalue_2 (`Texture2D.Blueprint_GetSizeX` Tex) _returnvalue))
  (`MaterialInstanceDynamic.SetTextureParameterValue` Mid "PoseA" Tex)
  (if (not (`KismetMathLibrary.IsZero2D` Offset))
    (`Widget.SetRenderTranslation` Image (`KismetMathLibrary.MakeVector2D` (- _x 105.0) (- (+ _y 485.0) (/ (`KismetMathLibrary.Conv_IntToDouble` _returnvalue) 3.0)))))
  (`Widget.SetVisibility` Image "Visible"))

(fn `TryLoadLevelFromPath`
  (params (Path :type String))
  (bind _boutsuccess (`LevelStreamingDynamic.LoadLevelInstance` Path))
  (if (not _boutsuccess)
    (`KismetSystemLibrary.PrintString` (`KismetStringLibrary.Concat_StrStr` "ERROR: Level at \"" Path "\" doesn't exist"))))

(fn `UserConstructionScript`)