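; Base Blueprint for player characters in events, providing shared helpers on top of its parent class.
; It forwards hidden-character comparisons against a local data index to the BPAtlEvtActorComp component.
; A reset function zeroes simulated locomotion velocity, stores the current actor location as the previous one and prints a debug string.
; Another enables in-editor animation updates on the costume, hair, face and main meshes.
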(event `self.ReceiveBeginPlay`
  (`parent.ReceiveBeginPlay`))

(fn `Compare To Hidden Character From Local Data`
  (params (LocalDataIndex :type Integer) (ConditionalValue :type Integer) (ConditionalType :type "EEvtConditionalBranchCompType Enum" :default "Equal"))
  (`AtlEvtActorComponent.CompareToHiddenCharacter` (`self.BPAtlEvtActorComp`) LocalDataIndex ConditionalValue ConditionalType))

(fn `ResetEvtLocomotionParams`
  (set `self.LocomotionSimVelocity` (0.0 0.0 0.0))
  (set `self.PrevTransformLocation` (`self.K2_GetActorLocation`))
  (`KismetSystemLibrary.PrintString` "Reset"))

(fn `SetUpdateAnimationInEditor`
  (`SkeletalMeshComponent.SetUpdateAnimationInEditor` (`self.CostumeMesh`) true)
  (`SkeletalMeshComponent.SetUpdateAnimationInEditor` (`self.HairMesh`) true)
  (`SkeletalMeshComponent.SetUpdateAnimationInEditor` (`self.FaceMesh`) true)
  (`SkeletalMeshComponent.SetUpdateAnimationInEditor` (`self.Mesh`) true))

(fn `UserConstructionScript`
  (`parent.UserConstructionScript`))