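; BP_BtlHumanBase is, by its name, a base Blueprint for human characters in battle, and it is almost entirely a stub.
; CreateCharacter takes a PlayerID but is empty, and ConvPlayerID always returns 0.
; The event graph holds only disabled default events, and the construction script just calls its parent.
; A helper named NotUsed calls SetGuard on the first BP_BtlPc01 actor it finds.
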(fn `ConvPlayerID`
  (params (PlayerID :type Integer))
  (returns (ConvPlayerID :type Integer))
  (return 0))

(fn `CreateCharacter`
  (params (PlayerID :type Integer)))

(fn `NotUsed`
  (bind _outactors (`GameplayStatics.GetAllActorsOfClass` "/Game/Xrd777/Blueprints/Battle/Players/Pc01/BP_BtlPc01.BP_BtlPc01_C"))
  (`self.SetGuard` (`|GetArrayItem` _outactors)))

(fn `UserConstructionScript`
  (`parent.UserConstructionScript`))